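; Player Blueprint that lets the user edit terrain with the mouse cursor.
; BeginPlay shows the cursor, and the click input deprojects the mouse into a long visibility line trace with debug drawing.
; When the trace hits a BP_TerrainActor, it calls Paint at the impact point, passing IsDigging as the removal flag.
; The A key toggles IsDigging to switch between adding and removing.
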(event `self.ReceiveBeginPlay`
  (set `PlayerController.bShowMouseCursor` true (`GameplayStatics.GetPlayerController` 0)))

(event `EnhancedInput|/Game/Blueprints/IA_Click`
  (params (ActionValue :type Boolean) (ElapsedSeconds :type "Float (double-precision)") (TriggeredSeconds :type "Float (double-precision)") (InputAction :type "InputAction Object Reference" :default "/Game/Blueprints/IA_Click.IA_Click"))
  (bind (_worldlocation _worlddirection) (`PlayerController.DeprojectMousePositionToWorld` (`GameplayStatics.GetPlayerController` 0)))
  (:`Triggered`
    (bind _outhit (`KismetSystemLibrary.LineTraceSingle` :`Start` _worldlocation :`End` (+ _worldlocation (* _worlddirection 50000.0)) :`TraceChannel` "TraceTypeQuery1" :`DrawDebugType` "ForDuration"))
    (bind (_bblockinghit _binitialoverlap _time _distance _location _impactpoint _normal _impactnormal _physmat _hitactor) (`GameplayStatics.BreakHitResult` _outhit))
    (bind _asbp_terrain_actor (cast `/Game/BP_TerrainActor` _hitactor))
    (`TerrainActor.Paint` _asbp_terrain_actor _impactpoint (`self.isDigging`))))

(event `Key|A`
  (params (Key :type "Key Structure"))
  (:`Pressed`
    (set `self.isDigging` (not (`self.isDigging`)))))

(fn `UserConstructionScript`)